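; BP_Follow_Cam is a camera actor that follows the side-scroller player character.
; On BeginPlay it casts player 0's character to BP_SideScrollerCharacter and stores the reference.
; Each Tick it snaps to the player's location plus an offset, without sweep or interpolation.
; It only moves while the player's Z is above zero, so it stops following when the player drops to that height or below.
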(event `self.ReceiveBeginPlay`
  ; Stores reference to the player
  (bind _asbp_side_scroller_character (cast `/Game/Blueprints/BP_SideScrollerCharacter` (`GameplayStatics.GetPlayerCharacter` 0)))
  (set `self.PlayerRef` _asbp_side_scroller_character))

(event `self.ReceiveTick`
  (params (DeltaSeconds :type "Float (single-precision)"))
  (bind _returnvalue (`self.K2_GetActorLocation` (`self.PlayerRef`)))
  ; set cam postion to players location + an offset
  (if (> (.z _returnvalue) 0.0)
    (`self.K2_SetActorLocation` (+ _returnvalue (`self.Offset`)))))

(fn `UserConstructionScript`)