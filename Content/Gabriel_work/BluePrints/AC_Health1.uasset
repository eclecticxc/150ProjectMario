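; Health component that applies damage to its owner and grants a temporary invincibility window after each non-lethal hit.
; TakeDamage ignores hits while invincible, otherwise subtracts from CurrentHealth and calls the death dispatcher at zero or below.
; Surviving hits start a delayed invincibility reset, call the damage-taken dispatcher and pass the new health to BP_GameInstance, which is not updated on death.
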(event `inviciblitycooldown`
  (`KismetSystemLibrary.Delay` 3.0)
  (set `self.IsInvincible` false))

(fn `Take Damage`
  (params (Damage :type "Float (double-precision)"))
  ; Controls overall health
  (if (not (`self.IsInvincible`))
    (bind _output_get (set `self.CurrentHealth` (- (`self.CurrentHealth`) Damage)))
    (if (<= _output_get 0.0)
      (`self.Ondeath `)
      (else
        (set `self.IsInvincible` true)
        (`self.inviciblitycooldown`)
        (`self.Damagetaken`)
        (bind _asbp_game_instance (cast `/Game/Sabrina_Work/BP_GameInstance` (`GameplayStatics.GetGameInstance`)))
        (`/Game/Sabrina_Work/BP_GameInstance.Gethealth` _asbp_game_instance (`self.CurrentHealth`))))))