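; AC_Health is a health component that applies damage to its owner and reports death.
; TakeDamage ignores hits while invincible, otherwise subtracts from CurrentHealth and calls the OnDeath dispatcher when health reaches zero or below.
; Each survived hit grants temporary invincibility, which a custom cooldown event clears after a fixed delay.
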(event `inviciblitycooldown`
  (`KismetSystemLibrary.Delay` 3.0)
  (set `self.IsInvincible` false))

(fn `Take Damage`
  (params (Damage :type "Float (double-precision)"))
  (if (not (`self.IsInvincible`))
    (bind _output_get (set `self.CurrentHealth` (- (`self.CurrentHealth`) Damage)))
    (if (<= _output_get 0.0)
      (`self.Ondeath `)
      (else
        (set `self.IsInvincible` true)
        (`self.inviciblitycooldown`)))))