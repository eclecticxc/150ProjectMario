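; A moving platform actor that shuttles back and forth between its placed location and an end point.
; BeginPlay stores both endpoints, reading the end from the StaticMesh component's world location, then hides that mesh so it acts as a marker.
; Tick sweeps the actor toward the current target with constant-speed interpolation at InterpSpeed and swaps targets on arrival.
; An empty Timeline and a second move node are left unconnected.
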(event `self.ReceiveBeginPlay`
  ; this helps control the platform to go to the starting point to the end point
  (set `self.StartPoint` (`self.K2_GetActorLocation`))
  (bind _output_get (set `self.EndPoint` (`SceneComponent.K2_GetComponentLocation` (`self.StaticMesh`))))
  (set `self.CurrentTarget` _output_get)
  (`SceneComponent.SetVisibility` (`self.StaticMesh`) false false))

(event `self.ReceiveTick`
  (params (DeltaSeconds :type "Float (single-precision)"))
  ; this controls the interpolation for the moving platform
  (`self.K2_SetActorLocation` (`KismetMathLibrary.VInterpTo_Constant` (`self.K2_GetActorLocation`) (`self.CurrentTarget`) (`GameplayStatics.GetWorldDeltaSeconds`) (`self.Interp Speed`)) true)
  (if (`KismetMathLibrary.EqualExactly_VectorVector` (`self.K2_GetActorLocation`) (`self.CurrentTarget`))
    (if (`KismetMathLibrary.EqualExactly_VectorVector` (`self.StartPoint`) (`self.CurrentTarget`))
      (set `self.CurrentTarget` (`self.EndPoint`))
      (else
        (set `self.CurrentTarget` (`self.StartPoint`))))))

(fn `UserConstructionScript`)