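; Goomba-style enemy character for a side-scroller that can be stomped by the player and deals contact damage.
; Tick sets movement velocity from Direction and Velocity, while BeginPlay reverses Direction only once, after a delay.
; When the player overlaps it and is inside StompZone, it destroys itself on the next tick.
; Enemy_damage_zone damages any overlapping actor with AC_Health, with no stomp check.
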(event `self.ReceiveActorBeginOverlap`
  (params (OtherActor :type "Actor Object Reference"))
  ; this is what makes the player destory the Goomba
  (cast `/Game/Blueprints/BP_SideScrollerCharacter` OtherActor)
  (for _array_element (`PrimitiveComponent.GetOverlappingActors` (`self.Stomp_zone`) null)
    (if (== (`GameplayStatics.GetObjectClass` _array_element) "/Game/Blueprints/BP_SideScrollerCharacter.BP_SideScrollerCharacter_C")
      (`|ExecutionSequence`
        (:`then_0`
          (`KismetSystemLibrary.DelayUntilNextTick`)
          (`self.K2_DestroyActor`))
        (:`then_1`
          (break))))))

(event `self.ReceiveBeginPlay`
  ; this is what makes the goomba move side to side
  (`self.AddMovementInput` (1.0 0.0 0.0))
  (`KismetSystemLibrary.Delay` 5.0)
  (set `self.Direction` (* (`self.Direction`) -1.0)))

(event `self.ReceiveTick`
  (params (DeltaSeconds :type "Float (single-precision)"))
  ; this is what makes the goomba move side to side
  (set `MovementComponent.Velocity` (* (`self.Direction`) (`self.Velocity`)) (`self.CharacterMovement`)))

(event `self.Enemy_damage_zone.OnComponentBeginOverlap`
  (params (OverlappedComponent :type "PrimitiveComponent Object Reference") (OtherActor :type "Actor Object Reference") (OtherComp :type "PrimitiveComponent Object Reference") (OtherBodyIndex :type Integer) (bFromSweep :type Boolean) (SweepResult :type "HitResult Structure (by ref)"))
  (bind _returnvalue (`self.GetComponentByClass` OtherActor "/Game/Gabriel_work/BluePrints/AC_Health.AC_Health_C"))
  ; This helps create the damge script for the Goomba
  (`/Engine/EditorBlueprintResources/StandardMacros.IsValid` _returnvalue
    (:`Is Valid`
      (`/Game/Gabriel_work/BluePrints/AC_Health.Take Damage` _returnvalue 1.0))))

(fn `UserConstructionScript`)