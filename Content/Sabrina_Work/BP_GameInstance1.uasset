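; Game instance that tracks the player's lives and coin score.
; A life-loss event decrements Lives and adds the WBP_GameOver widget to the viewport at zero or below.
; Coin pickups raise CoinValue, then grant one life when it reaches a milestone, which advances by CoinValuePerLife.
; Gethealth overwrites Lives with a truncated health value passed in.
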(event `CustomEvent`
  ; Reduce Lives and Check for Game Over.
  (bind _result (`/Engine/EditorBlueprintResources/StandardMacros.DecrementInt` (`self.Lives`))
    (:`  `
      (if (<= _result 0)
        (bind _returnvalue (`|CreateWidget` "/Game/Sabrina_Work/UI/WBP_GameOver.WBP_GameOver_C"))
        (`UserWidget.AddToViewport` _returnvalue 0)))))

(event `Add coinscore`
  (params (`Amt to add` :type Integer))
  ; Increase Coin Vaule by given amount
  (set `self.CoinValue` (+ `Amt to add` (`self.CoinValue`)))
  (`self.Updateslives`))

(event `Updateslives`
  ; Add 1 live for every 100 coin value are made
  (if (>= (`self.CoinValue`) (`self.Valuemilestone`))
    (set `self.Lives` (+ (`self.Lives`) 1))
    (set `self.Valuemilestone` (+ (`self.Valuemilestone`) (`self.Coin Value per Life`)))))

(event `Gethealth`
  (params (CurrentHealth :type "Float (double-precision)"))
  (set `self.Lives` (`KismetMathLibrary.FTrunc` CurrentHealth)))